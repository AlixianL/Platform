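; Key pickup actor that the third-person character collects by walking into it.
; On box overlap with BP_ThirdPersonCharacter, it sets the character's EnterIncolisionKey flag, clears its KeyActor reference and destroys itself.
; The end-overlap event does nothing; disconnected leftover chains hold earlier logic with French debug prints, including a hint to find a door to open.
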(event `self.BoxCollider.OnComponentBeginOverlap`
  (params (OverlappedComponent :type "PrimitiveComponent Object Reference") (OtherActor :type "Actor Object Reference") (OtherComp :type "PrimitiveComponent Object Reference") (OtherBodyIndex :type Integer) (bFromSweep :type Boolean) (SweepResult :type "HitResult Structure (by ref)"))
  (bind _asbp_third_person_character (cast `/Game/Blueprints/ThirdPersone_PB/BP_ThirdPersonCharacter` OtherActor))
  (set `/Game/Blueprints/ThirdPersone_PB/BP_ThirdPersonCharacter.EnterIncolisionKey?` true _asbp_third_person_character)
  (set `/Game/Blueprints/ThirdPersone_PB/BP_ThirdPersonCharacter.KeyActor` null _asbp_third_person_character)
  (`self.K2_DestroyActor` self))

(event `self.BoxCollider.OnComponentEndOverlap`
  (params (OverlappedComponent :type "PrimitiveComponent Object Reference") (OtherActor :type "Actor Object Reference") (OtherComp :type "PrimitiveComponent Object Reference") (OtherBodyIndex :type Integer))
  ; Useless
)

(fn `UserConstructionScript`)